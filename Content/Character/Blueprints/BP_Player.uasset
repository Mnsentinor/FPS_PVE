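; Player character Blueprint whose only logic is the OnShoot function for firing an assault rifle.
; Each shot is a hitscan line trace along the camera's forward vector, still drawing debug lines, that applies WeaponPower damage to the hit actor.
; The same function activates the muzzle flash, starts a camera shake and plays an attenuated gunshot sound at the player's location.
; BeginPlay and the construction script are empty.
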(event EventBeginPlay)

(fn ConstructionScript)

(fn OnShoot
  (bind _camera (Variables|Default|GetCamera))
  (bind _returnvalue (Transformation|GetWorldLocation _camera))
  (Components|Activation|Activate (Variables|Default|GetP_ChickenMaster_MuzzleFlash_01) true)
  (bind _outhit (Collision|LineTraceByChannel _returnvalue (+ _returnvalue (* (Math|Vector|GetForwardVector _camera) 1e+04)) "TraceTypeQuery3" false 0 "ForDuration" true "(R=1.000000,G=0.000000,B=0.000000,A=1.000000)" "(R=0.000000,G=1.000000,B=0.000000,A=1.000000)" 1.0))
  (Game|Damage|ApplyDamage (.hitactor _outhit) (Variables|Default|GetWeaponPower) 0 0)
  (CameraShakes|StartCameraShake (Game|GetPlayerCameraManager 0) "/Game/Weapen/BP_AK_Shake.BP_AK_Shake_C" 1.0 "CameraLocal" "0, 0, 0")
  (Audio|PlaySoundatLocation "/Game/Weapen/Sounds/Assault_Rifle_Shot_03_Cue.Assault_Rifle_Shot_03_Cue" (Transformation|GetActorLocation self) "0, 0, 0" 1.0 1.0 0.0 "/Game/Weapen/Sounds/GunShotSoundAuttenuation.GunShotSoundAuttenuation" 0 0))