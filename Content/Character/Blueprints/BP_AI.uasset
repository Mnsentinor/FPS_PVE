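; BP_AI is an AI shooter that fires automatically while something overlaps its Box trigger, with no filter on the overlapping actor.
; Begin overlap sets IsFire and starts a short Delay loop calling OnShoot, until any end overlap clears the flag.
; OnShoot activates the muzzle flash, line-traces forward from the Camera with debug drawing, applies damage to the hit actor, and plays an attenuated rifle sound.
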(event OnComponentBeginOverlap(Box)
  (params (OverlappedComponent :type Primitive%20Component%20Object%20Reference) (OtherActor :type Actor%20Object%20Reference) (OtherComp :type Primitive%20Component%20Object%20Reference) (OtherBodyIndex :type Integer) (bFromSweep :type Boolean) (SweepResult :type Hit%20Result%20Structure%20%28by%20ref%29))
  (bind _output_get (Variables|Default|SetIsFire true))
  (if _output_get :!label _label
    (CallFunction|OnShoot)
    (Utilities|FlowControl|Delay 0.1)
    (goto _label)))

(event OnComponentEndOverlap(Box)
  (params (OverlappedComponent :type Primitive%20Component%20Object%20Reference) (OtherActor :type Actor%20Object%20Reference) (OtherComp :type Primitive%20Component%20Object%20Reference) (OtherBodyIndex :type Integer))
  (Variables|Default|SetIsFire false))

(fn ConstructionScript)

(fn OnShoot
  (bind _camera (Variables|Default|GetCamera))
  (bind _returnvalue (Transformation|GetWorldLocation _camera))
  (Components|Activation|Activate (Variables|Default|GetP_ChickenMaster_MuzzleFlash_01) true)
  (bind _outhit (Collision|LineTraceByChannel _returnvalue (+ _returnvalue (* (Math|Vector|GetForwardVector _camera) 1e+04)) "TraceTypeQuery3" false 0 "ForDuration" true "(R=1.000000,G=0.000000,B=0.000000,A=1.000000)" "(R=0.000000,G=1.000000,B=0.000000,A=1.000000)" 1.0))
  (Game|Damage|ApplyDamage (.hitactor _outhit) 1e+02 0 0)
  (Audio|PlaySoundatLocation "/Game/Weapen/Sounds/Assault_Rifle_Shot_03_Cue.Assault_Rifle_Shot_03_Cue" (Transformation|GetActorLocation self) "0, 0, 0" 1.0 1.0 0.0 "/Game/Weapen/Sounds/GunShotSoundAuttenuation.GunShotSoundAuttenuation" 0 0))