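; Player controller that turns movement, look, run, jump and shoot input into actions on its ControlledPlayer character.
; Movement follows the capsule's facing, look input drives controller yaw and pitch (storing yaw input in ZAxisOscillation), and Run switches max walk speed.
; Shooting casts to BP_Player and sets IsFire, calling OnShoot in a delayed loop until release clears the flag, giving automatic fire.
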(event EventBeginPlay)

(event EventTick
  (params (DeltaSeconds :type Float%20%28single-precision%29)))

(event Input|ActionEvents|InputActionShoot
  (params (Key :type Key%20Structure :default "None"))
  (bind _controlledplayer (Variables|Default|GetControlledPlayer))
  (:Pressed
    (bind _asbp_player (Utilities|Casting|CastToBP_Player _controlledplayer))
    (bind _output_get (Variables|/Script/FPS_PVE.FPS_PVECharacter|SetIsFire _asbp_player true))
    (if _output_get :!label _label
      (Default|OnShoot _asbp_player)
      (Utilities|FlowControl|Delay 0.1)
      (goto _label)))
  (:Released
    (bind _asbp_player_2 (Utilities|Casting|CastToBP_Player _controlledplayer))
    (Variables|/Script/FPS_PVE.FPS_PVECharacter|SetIsFire _asbp_player_2 false)))

(event Input|ActionEvents|InputActionJump
  (params (Key :type Key%20Structure :default "None"))
  (bind _controlledplayer (Variables|Default|GetControlledPlayer))
  (:Pressed
    (Character|Jump _controlledplayer))
  (:Released
    (Character|StopJumping _controlledplayer)))

(event Input|ActionEvents|InputActionRun
  (params (Key :type Key%20Structure :default "None"))
  (bind _controlledplayer (Variables|Default|GetControlledPlayer))
  (bind _charactermovement (Variables|/Script/Engine.Character|GetCharacterMovement _controlledplayer))
  (:Pressed
    (Variables|/Script/Engine.CharacterMovementComponent|SetMaxWalkSpeed _charactermovement 8e+02))
  (:Released
    (Variables|/Script/Engine.CharacterMovementComponent|SetMaxWalkSpeed _charactermovement 4e+02)))

(event Input|AxisEvents|InputAxisWS
  (params (AxisValue :type Float%20%28single-precision%29))
  (Pawn|Input|AddMovementInput (Variables|Default|GetControlledPlayer) (Math|Vector|GetForwardVector (Transformation|GetWorldRotation (Variables|/Script/Engine.Character|GetCapsuleComponent (Variables|Default|GetControlledPlayer)))) AxisValue false))

(event Input|AxisEvents|InputAxisAD
  (params (AxisValue :type Float%20%28single-precision%29))
  (Pawn|Input|AddMovementInput (Variables|Default|GetControlledPlayer) (Math|Vector|GetRightVector (Transformation|GetWorldRotation (Variables|/Script/Engine.Character|GetCapsuleComponent (Variables|Default|GetControlledPlayer)))) AxisValue false))

(event Input|AxisEvents|InputAxisUD
  (params (AxisValue :type Float%20%28single-precision%29))
  (Pawn|Input|AddControllerPitchInput (Variables|Default|GetControlledPlayer) AxisValue))

(event Input|AxisEvents|InputAxisLR
  (params (AxisValue :type Float%20%28single-precision%29))
  (Pawn|Input|AddControllerYawInput (Variables|Default|GetControlledPlayer) AxisValue)
  (Variables|Default|SetZ_AxisOscillation AxisValue))

(fn ConstructionScript)